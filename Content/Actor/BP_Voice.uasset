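; BP_Voice is an actor that advances through a sequence of voice sounds as missions complete.
; From BeginPlay it listens on the ComplateMission gameplay message channel with exact matching and calls SetNextVoice for each message.
; SetNextVoice stops the Audio component, increments CurSoundIndex, and plays that SoundArray entry from the start if it is valid.
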(event `self.ReceiveBeginPlay`
  (`|AsyncAction_ListenForGameplayMessages` (struct :`TagName` "ComplateMission")
    (:`OnMessageReceived`
      (`self.SetNextVoice`))))

(fn `SetNextVoice`
  (bind _audio (`self.Audio`))
  (`AudioComponent.Stop` _audio)
  (bind _result (`/Engine/EditorBlueprintResources/StandardMacros.IncrementInt` (`self.CurSoundIndex`))
    (:`  `
      (bind _output (`|GetArrayItem` (`self.SoundArray`) _result))
      (`/Engine/EditorBlueprintResources/StandardMacros.IsValid` _output
        (:`Is Valid`
          (`AudioComponent.SetSound` _audio _output)
          (`AudioComponent.Play` _audio 0.0))))))

(fn `UserConstructionScript`)