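; BP_StorageAnswerManager is an actor that judges whether a selected storage area matches the current DG type.
; On BeginPlay it listens on the Select.StorageArea gameplay message channel and compares the payload's DGType against CurDGType.
; A match broadcasts Event.Success and Event.SceneEnd, while a mismatch broadcasts Event.Failed with a wrong-loading-location text.
; Both outcomes also print a Korean debug string.
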(event `self.ReceiveBeginPlay`
  (bind _returnvalue (subsystem `GameplayMessageSubsystem`))
  (bind (_asynctaskproxy _actualchannel _payload) (`|AsyncAction_ListenForGameplayMessages` (struct :`TagName` "Select.StorageArea") "/Game/Widget/AreaText/ST_SelectStorageArea.ST_SelectStorageArea")
    (:`OnMessageReceived`
      (if (`|EnumEquality` (`self.CurDGType`) (`.DGType_2_179B9C7D4A27C3EA8D81EE839AD1A5E1` (break `/Game/Widget/AreaText/ST_SelectStorageArea` _payload)))
        (`KismetSystemLibrary.PrintString` "올바른 선택입니다.")
        (`GameplayMessageSubsystem.K2_BroadcastMessage` _returnvalue (struct :`TagName` "Event.Success") (make `/Game/Widget/Result/ST_SuccessList` ""))
        (`GameplayMessageSubsystem.K2_BroadcastMessage` _returnvalue (struct :`TagName` "Event.SceneEnd") (make `/Game/Actor/ST_SceneEnd` "NewEnumerator2"))
        (else
          (`KismetSystemLibrary.PrintString` "잠깐 더 안전한 어쩌구")
          (`GameplayMessageSubsystem.K2_BroadcastMessage` _returnvalue (struct :`TagName` "Event.Failed") (make `/Game/Widget/Result/ST_FailedList` "잘못된 장소에 적재함")))))))

(fn `UserConstructionScript`)