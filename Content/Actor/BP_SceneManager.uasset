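; Scene manager actor that advances the game through three sequential scenes and then an end state, using Gameplay Message Subsystem channels.
; On BeginPlay it starts the current scene and listens for scene-end messages, whose scene type picks the next scene to start.
; Starting each numbered scene broadcasts its scene-specific start message and a play-sound message with a fire cue, while the end state broadcasts nothing.
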(event `self.ReceiveBeginPlay`
  (`self.StartScene`)
  (bind (_asynctaskproxy _actualchannel _payload) (`|AsyncAction_ListenForGameplayMessages` (struct :`TagName` "Event.SceneEnd") "/Game/Actor/ST_SceneEnd.ST_SceneEnd")
    (:`OnMessageReceived`
      (`self.EndScene` (`.SceneType_5_7CA14D0940BACB6CCDA1E09E85D70358` (break `/Game/Actor/ST_SceneEnd` _payload))))))

(fn `EndScene`
  (params (EndSceneType :type "/Game/Enum/SceneType Enum" :default "NewEnumerator0"))
  (locals (SceneEndSound :type "SoundCue Object Reference"))
  (switch `/Game/Enum/SceneType` EndSceneType
    (:`NewEnumerator0`
      (set `self.CurScene` "NewEnumerator1"))
    (:`NewEnumerator1`
      (set `self.CurScene` "NewEnumerator2"))
    (:`NewEnumerator2`
      (set `self.CurScene` "NewEnumerator3" :!label _label))
    (:`NewEnumerator3`
      (goto _label)))
  (`self.StartScene`))

(fn `StartScene`
  (locals (Channel :type "GameplayTag Structure" :default (struct)) (SceneStartSound :type "SoundCue Object Reference" :default "/Script/Engine.SoundCue'/Game/VRTemplate/Audio/Fire_Cue.Fire_Cue'"))
  (bind _returnvalue (subsystem `GameplayMessageSubsystem`))
  (switch `/Game/Enum/SceneType` (`self.CurScene`)
    (:`NewEnumerator0`
      (set `local.Channel` (struct :`TagName` "Event.SceneStart.One"))
      (set `local.SceneStartSound` "/Game/VRTemplate/Audio/Fire_Cue.Fire_Cue")
      (`GameplayMessageSubsystem.K2_BroadcastMessage` _returnvalue (`local.Channel`) (make `/Game/Actor/ST_SceneStart` null) :!label _label)
      (`GameplayMessageSubsystem.K2_BroadcastMessage` _returnvalue (struct :`TagName` "Event.PlaySound") (make `/Game/Actor/ST_Speaker` (`local.SceneStartSound`))))
    (:`NewEnumerator1`
      (set `local.Channel` (struct :`TagName` "Event.SceneStart.Two"))
      (set `local.SceneStartSound` "/Game/VRTemplate/Audio/Fire_Cue.Fire_Cue")
      (goto _label))
    (:`NewEnumerator2`
      (set `local.Channel` (struct :`TagName` "Event.SceneStart.Three"))
      (set `local.SceneStartSound` "/Game/VRTemplate/Audio/Fire_Cue.Fire_Cue")
      (goto _label))
    (:`NewEnumerator3`
      (set `local.Channel` (struct)))))

(fn `UserConstructionScript`)