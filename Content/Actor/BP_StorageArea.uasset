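; BP_StorageArea is an interactable storage area actor that can be highlighted and selected.
; Ray hit start and end events set and clear an outline overlay material on its Plane mesh.
; Interact broadcasts a Select.StorageArea message through the Gameplay Message Subsystem, carrying the area's DGType, so the actor needs no direct reference to listeners.
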(event `/Game/Interface/BPI_InteractAble.RayHitStart`
  (`MeshComponent.SetOverlayMaterial` (`self.Plane`) (`self.OutLineMat`)))

(event `/Game/Interface/BPI_InteractAble.RayHitEnd`
  (`MeshComponent.SetOverlayMaterial` (`self.Plane`) null))

(event `/Game/Interface/BPI_InteractAble.Interact`
  (`GameplayMessageSubsystem.K2_BroadcastMessage` (subsystem `GameplayMessageSubsystem`) (struct :`TagName` "Select.StorageArea") (make `/Game/Widget/AreaText/ST_SelectStorageArea` (`self.DGType`))))

(fn `UserConstructionScript`)