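; BP_Signs is an interactable sign actor that reveals a checklist widget.
; The widget is hidden at BeginPlay and shown on Interact, with no hiding afterward.
; Ray hit start and end events toggle an outline overlay material on the Plane.
; ReflashCheckList, not called within this asset, wraps each CheckListData entry in a BP_ChecklistData object, appends it to ChecklistDatas without clearing, then calls SetCheckList on WBP_Checklist.
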(event `self.ReceiveBeginPlay`
  (`SceneComponent.SetVisibility` (`self.Widget`) false false))

(event `/Game/Interface/BPI_InteractAble.Interact`
  (`SceneComponent.SetVisibility` (`self.Widget`) true false))

(event `/Game/Interface/BPI_InteractAble.RayHitStart`
  (`MeshComponent.SetOverlayMaterial` (`self.Plane`) (`self.OutLineMat`)))

(event `/Game/Interface/BPI_InteractAble.RayHitEnd`
  (`MeshComponent.SetOverlayMaterial` (`self.Plane`) null))

(fn `ReflashCheckList`
  (locals (ChecklistDatas :type "Array of /Game/Widget/Checklist/BP_ChecklistData Object Reference"))
  (for _array_element (`self.CheckListData`)
    (bind _returnvalue (`|GenericCreateObject` "/Game/Widget/Checklist/BP_ChecklistData.BP_ChecklistData_C"))
    (`/Engine/EditorBlueprintResources/StandardMacros.IsValid` _returnvalue
      (:`Is Valid`
        (set `/Game/Widget/Checklist/BP_ChecklistData.Checklist` _array_element _returnvalue)
        (`KismetArrayLibrary.Array_Add` (`local.ChecklistDatas`) _returnvalue))))
  (bind _aswbp_checklist (cast `/Game/Widget/Checklist/WBP_Checklist` (`WidgetComponent.GetWidget` (`self.Widget`))))
  (`/Game/Widget/Checklist/WBP_Checklist.SetCheckList` :`self` _aswbp_checklist))

(fn `UserConstructionScript`)